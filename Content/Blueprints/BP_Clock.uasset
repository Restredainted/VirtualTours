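; BP_Clock is a clock Blueprint with hour, minute and second hand components, currently left non-functional.
; BeginPlay leads only to an empty Sequence, and both the custom event and construction script do nothing.
; Disconnected nodes would set each hand's relative rotation to zero, with a debug print for the minute hand, but none of them run.
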(event `CustomEvent`)

(event `self.ReceiveBeginPlay`
  (`|ExecutionSequence`))

(fn `UserConstructionScript`)