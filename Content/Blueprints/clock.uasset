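; Clock actor that shows the real system time on hour, minute and second hand components.
; From BeginPlay, a one-second Delay loop reads Now and sets each hand's relative pitch.
; The hour hand also creeps with the current minute, and angles are negated to set the turn direction.
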(event `self.ReceiveBeginPlay`
  (bind (_year _month _day _hour _minute _second) (`KismetMathLibrary.BreakDateTime` (`KismetMathLibrary.Now`)))
  (`SceneComponent.K2_SetRelativeRotation` (`self.Clock_Hour_Hand`) (`KismetMathLibrary.MakeRotator` 0.0 (* (+ (* _hour 30.0) (/ _minute 2)) -1.0)) false false :!label _label)
  (`SceneComponent.K2_SetRelativeRotation` (`self.Clock_Minutes_Hand`) (`KismetMathLibrary.MakeRotator` 0.0 (* _minute -6.0)) false false)
  (`SceneComponent.K2_SetRelativeRotation` (`self.Clock_Seconds_Hand`) (`KismetMathLibrary.MakeRotator` 0.0 (* _second -6.0)) false false)
  (`KismetSystemLibrary.Delay` 1.0)
  (goto _label))

(fn `UserConstructionScript`)