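; Sliding double door that opens when a VR-Character or BP_FirstPersonCharacter overlaps it and closes 1.5 seconds after overlap ends.
; An opening timeline and a separate closing timeline, played in reverse, feed DoorAction, which moves both panels oppositely along local Y.
; The Lerp squares the timeline value, and Y ignores the cached starting position while X and Z keep it.
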(event `self.ReceiveBeginPlay`
  (set `self.L_Door_Initial_Position` (`SceneComponent.RelativeLocation` (`self.StaticMesh_Door_L`)))
  (set `self.R_Door_Initial_Position` (`SceneComponent.RelativeLocation` (`self.StaticMesh_Door_R`))))

(event `self.ReceiveActorBeginOverlap`
  (params (OtherActor :type "Actor Object Reference"))
  (cast `/Game/VR-Character/VR-Character` OtherActor
    (:`then`
      (bind (_direction _doormovement) (`Timeline|DoorMovement` :!via `PlayFromStart` :!label _label)
        (:`Update`
          (`self.DoorAction` _doormovement))))
    (:`CastFailed`
      (cast `/Game/FirstPerson/Blueprints/BP_FirstPersonCharacter` OtherActor)
      (goto _label :!via `PlayFromStart`))))

(event `self.ReceiveActorEndOverlap`
  (params (OtherActor :type "Actor Object Reference"))
  (cast `/Game/VR-Character/VR-Character` OtherActor
    (:`then`
      _)
    (:`CastFailed`
      (cast `/Game/FirstPerson/Blueprints/BP_FirstPersonCharacter` OtherActor)))
  (`KismetSystemLibrary.Delay` 1.5)
  (bind (_direction _doormovement) (`Timeline|DoorMovement_Close` :!via `ReverseFromEnd`)
    (:`Update`
      (`self.DoorAction` _doormovement))))

(event `DoorAction`
  (params (OffsetValue :type "Float (double-precision)"))
  (bind _returnvalue (`KismetMathLibrary.Lerp` 0.0 (`self.OffsetValue`) OffsetValue))
  (`|ExecutionSequence`
    (:`then_0`
      (`SceneComponent.K2_SetRelativeLocation` (`self.StaticMesh_Door_L`) (`KismetMathLibrary.MakeVector` (.x (`self.L_Door_Initial_Position`)) (* _returnvalue -1.0) (.z (`self.L_Door_Initial_Position`))) false false))
    (:`then_1`
      (`SceneComponent.K2_SetRelativeLocation` (`self.StaticMesh_Door_R`) (`KismetMathLibrary.MakeVector` (.x (`self.R_Door_Initial_Position`)) _returnvalue (.z (`self.R_Door_Initial_Position`))) false false))))

(fn `UserConstructionScript`)