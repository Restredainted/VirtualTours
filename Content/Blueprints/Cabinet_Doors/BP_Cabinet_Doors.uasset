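; BP_Cabinet_Doors is a double-door cabinet that swings open and closed automatically as a player pawn comes and goes.
; Entering the Open_Range trigger plays a timeline, and leaving the separate Close_Range trigger reverses it.
; The timeline's Door track, scaled by DoorOpenAngle, yaws the left and right meshes in opposite directions.
; A chain of casts limits triggering to third-person, first-person and two VR player classes.
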(event `self.Open_Range.OnComponentBeginOverlap`
  (params (OverlappedComponent :type "PrimitiveComponent Object Reference") (OtherActor :type "Actor Object Reference") (OtherComp :type "PrimitiveComponent Object Reference") (OtherBodyIndex :type Integer) (bFromSweep :type Boolean) (SweepResult :type "HitResult Structure (by ref)"))
  (`KismetSystemLibrary.PrintString` "OpenDoor")
  (cast `/Game/ThirdPerson/Blueprints/BP_ThirdPersonCharacter` OtherActor
    (:`then`
      (bind (_direction _door) (`Timeline|Timeline` :!label _label)
        (:`Update`
          (bind _returnvalue (* _door (`self.DoorOpenAngle`)))
          (`SceneComponent.K2_SetRelativeRotation` (`self.StaticMesh_Left`) (`KismetMathLibrary.MakeRotator` 0.0 0.0 _returnvalue) false false)
          (`SceneComponent.K2_SetRelativeRotation` (`self.StaticMesh_Right`) (`KismetMathLibrary.MakeRotator` 0.0 0.0 (* _returnvalue -1.0)) false false))))
    (:`CastFailed`
      (cast `/Game/FirstPerson/Blueprints/BP_FirstPersonCharacter` OtherActor
        (:`then`
          (goto _label))
        (:`CastFailed`
          (cast `/Game/VR-Character/VR-Character` OtherActor
            (:`then`
              (goto _label))
            (:`CastFailed`
              (cast `/Game/VRTemplate/Blueprints/VRPawn` OtherActor)
              (goto _label))))))))

(event `self.Close_Range.OnComponentEndOverlap`
  (params (OverlappedComponent :type "PrimitiveComponent Object Reference") (OtherActor :type "Actor Object Reference") (OtherComp :type "PrimitiveComponent Object Reference") (OtherBodyIndex :type Integer))
  (cast `/Game/ThirdPerson/Blueprints/BP_ThirdPersonCharacter` OtherActor
    (:`then`
      (goto _label :!via `Reverse`))
    (:`CastFailed`
      (cast `/Game/FirstPerson/Blueprints/BP_FirstPersonCharacter` OtherActor
        (:`then`
          (goto _label :!via `Reverse`))
        (:`CastFailed`
          (cast `/Game/VR-Character/VR-Character` OtherActor
            (:`then`
              (goto _label :!via `Reverse`))
            (:`CastFailed`
              (cast `/Game/VRTemplate/Blueprints/VRPawn` OtherActor)
              (goto _label :!via `Reverse`))))))))

(fn `UserConstructionScript`)